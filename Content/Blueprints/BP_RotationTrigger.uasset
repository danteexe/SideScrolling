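; BP_RotationTrigger is a trigger that turns the player's camera spring arm and redefines their axis vectors on overlap.
; When BP_Player enters, it copies its XAxisVector and RightVector onto the player, then restarts RotationTimeline.
; Each timeline update lerps SpringArm1's world rotation toward the trigger's Rotation, re-reading the arm's current target rotation as the start, so the blend compounds rather than following the curve directly.
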(event OnComponentBeginOverlap(Trigger)
  (params (OverlappedComponent :type Primitive%20Component%20Object%20Reference) (OtherActor :type Actor%20Object%20Reference) (OtherComp :type Primitive%20Component%20Object%20Reference) (OtherBodyIndex :type Integer) (bFromSweep :type Boolean) (SweepResult :type Hit%20Result%20Structure%20%28by%20ref%29))
  (bind _asbp_player (Utilities|Casting|CastToBP_Player OtherActor))
  (Variables|/Game/Blueprints/BP_Player.BP_Player_C|SetXAxisVector _asbp_player (Variables|Default|GetXAxisVector))
  (Variables|/Game/Blueprints/BP_Player.BP_Player_C|SetRightVector _asbp_player (Variables|Default|GetRightVector))
  (bind _rotationtrack (Timeline|RotationTimeline PlayFromStart)
    (:Update
      (Transformation|SetWorldRotation (Variables|/Game/Blueprints/BP_Player.BP_Player_C|GetSpringArm1 _asbp_player) (Math|Rotator|Lerp(Rotator) (Class|SpringArmComponent|GetTargetRotation (Variables|/Game/Blueprints/BP_Player.BP_Player_C|GetSpringArm1 _asbp_player)) (Variables|Default|GetRotation) _rotationtrack) false false))))

(event EventBeginPlay)

(event Collision|EventActorBeginOverlap
  (params (OtherActor :type Actor%20Object%20Reference)))

(event EventTick
  (params (DeltaSeconds :type Float%20%28single-precision%29)))

(fn ConstructionScript)