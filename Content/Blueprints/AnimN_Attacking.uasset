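; AnimN_Attacking is an animation notify state that deals melee damage during a character's attack animation.
; Each tick, it casts the mesh owner to BP_CharacterBase and capsule-traces between the weapon mesh's BeginSocket and EndSocket on the Camera channel, with debug drawing.
; Any blocking hit receives the character's Damage, with no tracking of already-hit actors, so one swing can damage a target repeatedly.
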(fn ReceivedNotifyTick
  (params (MeshComp :type Skeletal%20Mesh%20Component%20Object%20Reference) (Animation :type Anim%20Sequence%20Base%20Object%20Reference) (FrameDeltaTime :type Float%20%28single-precision%29))
  (CallFunction|FireTrace MeshComp)
  (return false))

(fn FireTrace
  (params (Mesh%20Component :type Scene%20Component%20Object%20Reference))
  (bind _asbp_character_base (CallFunction|GetasCharacterBase Mesh%20Component))
  (bind _weaponmesh (Variables|/Game/Blueprints/BP_CharacterBase.BP_CharacterBase_C|GetWeaponMesh _asbp_character_base))
  (bind (_startlocation _endlocation) (CallFunction|GetLocations _weaponmesh))
  (bind _outhit (Collision|CapsuleTraceByChannel _weaponmesh _startlocation _endlocation 12.0 1.0 "TraceTypeQuery2" false 0 "ForDuration"))
  (if (.bBlockingHit (Collision|BreakHitResult _outhit))
    (Game|Damage|ApplyDamage (.HitActor (Collision|BreakHitResult _outhit)) (Variables|/Game/Blueprints/BP_CharacterBase.BP_CharacterBase_C|GetDamage _asbp_character_base) 0 0)))

(fn GetasCharacterBase
  (params (MeshComponent :type Actor%20Component%20Object%20Reference))
  (bind _asbp_character_base (Utilities|Casting|CastToBP_CharacterBase (Components|GetOwner MeshComponent)))
  (return _asbp_character_base))

(fn GetLocations
  (params (Object :type Scene%20Component%20Object%20Reference))
  (return (Transformation|GetSocketLocation Object "BeginSocket") (Transformation|GetSocketLocation Object "EndSocket")))